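; BP_Weaponspawner is a placed actor that spawns the player's selected weapon at its own transform when play begins.
; It reads WeaponType from the GI_VRProject game instance and switches to spawn a Seung Jar gun, musket or cannon actor.
; The musket spawns with an extra 90-degree rotation offset, while the other weapons use the spawner's transform directly.
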(event EventBeginPlay
  (bind _asgi_vrproject (Utilities|Casting|CastToGI_VRProject (Game|GetGameInstance)))
  (Variables|Default|SetSpawnTransform (Transformation|GetActorTransform self))
  (switch Utilities|FlowControl|Switch|SwitchonE_Weapons (Variables|/Game/BowAndMusket/Blueprints/GI_VRProject.GI_VRProject_C|GetWeaponType _asgi_vrproject)
    (:NewEnumerator0
      (Game|SpawnActorfromClass "/Game/BowAndMusket/Weapons/Blueprints/BP_SeungJarGun.BP_SeungJarGun_C" (Variables|Default|GetSpawnTransform) "Undefined" 0 0)
      (Development|PrintString "스폰"))
    (:NewEnumerator2
      (Game|SpawnActorfromClass "/Game/BowAndMusket/Weapons/Blueprints/BP_Musket.BP_Musket_C" (Math|Transform|MakeTransform (.Location (Math|Transform|BreakTransform (Variables|Default|GetSpawnTransform))) (Math|Rotator|CombineRotators (.Rotation (Math|Transform|BreakTransform (Variables|Default|GetSpawnTransform))) "0,90.000000, 0") (.Scale (Math|Transform|BreakTransform (Variables|Default|GetSpawnTransform)))) "Undefined" 0 0))
    (:NewEnumerator3
      (Game|SpawnActorfromClass "/Game/BowAndMusket/Weapons/Blueprints/BP_Cannon.BP_Cannon_C" (Variables|Default|GetSpawnTransform) "Undefined" 0 0))))

(fn ConstructionScript)