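; Spawner actor for the VR weapon experience that places either a gunpowder (BP_Powder) or mud wad (BP_Mud) actor at its own transform.
; On BeginPlay it reads the weapon type from GI_VRProject and spawns the object selected by ObjectTypeToSpawn.
; Seung Jar Gun and Musket share default spawns, while Cannon Ball overrides the spawned mesh scale.
; RespawnAll repeats the spawn only when the stored actor reference is no longer valid.
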(event Custom|RespawnAll
  ;[1 1 1] 전체 리스폰
  (switch Utilities|FlowControl|Switch|SwitchonE_PhysicalObjectType (Variables|Default|GetObjectTypeToSpawn)
    (:NewEnumerator0
      (CallFunction|SpawnPowder))
    (:NewEnumerator1
      (CallFunction|SpawnMud))))

(event Custom|SpawnMud
  (bind _spawntransform (Variables|Default|GetSpawnTransform))
  ;[1 1 1] 맵에 토격 스폰
  (Utilities|IsValid (Variables|Default|GetSpawnedMud)
    (:Is%20Not%20Valid
      (switch Utilities|FlowControl|Switch|SwitchonE_Weapons (Variables|Default|GetWeapon%20Type)
        (:NewEnumerator0
          (bind _returnvalue (Game|SpawnActorfromClass "/Game/BowAndMusket/Weapons/Blueprints/NotGuns/BP_Mud.BP_Mud_C" _spawntransform "AlwaysSpawn" 0 0 :!label _label))
          (Variables|Default|SetSpawnedMud _returnvalue))
        (:NewEnumerator2
          (goto _label))
        (:NewEnumerator3
          (bind _returnvalue_2 (Game|SpawnActorfromClass "/Game/BowAndMusket/Weapons/Blueprints/NotGuns/BP_Mud.BP_Mud_C" _spawntransform "AlwaysSpawn" 0 0))
          (Transformation|SetWorldScale3D (Variables|/Game/BowAndMusket/Weapons/Blueprints/NotGuns/BP_Mud.BP_Mud_C|GetMudBase _returnvalue_2) "0.150000,0.150000,0.150000")
          (Variables|Default|SetSpawnedMud _returnvalue_2))))))

(event Custom|SpawnPowder
  (bind _spawntransform (Variables|Default|GetSpawnTransform))
  ;[1 1 1] 맵에 화약 스폰
  (Utilities|IsValid (Variables|Default|GetSpawnedPowder)
    (:Is%20Not%20Valid
      (switch Utilities|FlowControl|Switch|SwitchonE_Weapons (Variables|Default|GetWeapon%20Type)
        (:NewEnumerator0
          (bind _returnvalue (Game|SpawnActorfromClass "/Game/BowAndMusket/Weapons/Blueprints/NotGuns/BP_Powder.BP_Powder_C" _spawntransform "AlwaysSpawn" 0 0 :!label _label))
          (Variables|Default|SetSpawnedPowder _returnvalue))
        (:NewEnumerator2
          (goto _label))
        (:NewEnumerator3
          (bind _returnvalue_2 (Game|SpawnActorfromClass "/Game/BowAndMusket/Weapons/Blueprints/NotGuns/BP_Powder.BP_Powder_C" _spawntransform "AlwaysSpawn" 0 0))
          (Transformation|SetWorldScale3D (Variables|/Game/BowAndMusket/Weapons/Blueprints/NotGuns/BP_Powder.BP_Powder_C|GetPowderBase _returnvalue_2) "1.000000,1.000000,1.000000")
          (Variables|Default|SetSpawnedPowder _returnvalue_2))))))

(event EventBeginPlay
  ;[1 1 1] 현재 체험 무기 종류를 가져온다
  (bind _asgi_vrproject (Utilities|Casting|CastToGI_VRProject (Game|GetGameInstance)))
  (Variables|Default|SetSpawnTransform (Transformation|GetActorTransform self))
  (Variables|Default|SetWeapon%20Type (Variables|/Game/BowAndMusket/Blueprints/GI_VRProject.GI_VRProject_C|GetWeaponType _asgi_vrproject))
  ;[1 1 1] 스폰할 오브젝트 결정
  (switch Utilities|FlowControl|Switch|SwitchonE_PhysicalObjectType (Variables|Default|GetObjectTypeToSpawn)
    (:NewEnumerator0
      (CallFunction|SpawnPowder))
    (:NewEnumerator1
      (CallFunction|SpawnMud))))

(fn ConstructionScript)