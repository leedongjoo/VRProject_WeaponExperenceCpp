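; Game mode for the bow and musket VR game that picks the player's spawn point and the map matching the platform.
; The ChoosePlayerStart override reads InitialStart from GI_VRProject, returning the "InitialStart"-tagged PlayerStart on a first start, otherwise a differently tagged one near the weapon selector.
; MapSelectByPlatform reads the game instance's Platform and returns either the PC or mobile map.
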(fn ConstructionScript)

(fn ChoosePlayerStart
  (params (Player :type Controller%20Object%20Reference))
  ;[1 1 1] 전역 변수 Initial Start 사용
  (bind _asgi_vrproject (Utilities|Casting|CastToGI_VRProject (Game|GetGameInstance)))
  (bind _outactors (Actor|GetAllActorsOfClass "/Script/Engine.PlayerStart"))
  (for _array_element _outactors
    (if (Variables|/Game/BowAndMusket/Blueprints/GI_VRProject.GI_VRProject_C|GetInitialStart _asgi_vrproject)
      ;[1 1 1] Initial Start가 트루라면 시작 포인트에서 스폰
      (if (Utilities|Name|Equal(Name) (Variables|/Script/Engine.PlayerStart|GetPlayerStartTag _array_element) "InitialStart")
        (return _array_element))
      (else
        ;[1 1 1] 한번이라도 무기를 체험했다면 무기 선택기와 가까운 곳에서 스폰
        (if (Utilities|Name|NotEqual(Name) (Variables|/Script/Engine.PlayerStart|GetPlayerStartTag _array_element) "InitialStart")
          (return _array_element))))))

(fn MapSelectbyPlatform
  (bind _asgi_vrproject (Utilities|Casting|CastToGI_VRProject (Game|GetGameInstance))) ; 인터페이스의 플렛폼 정보를 가져온다
  (Utilities|IsValid _asgi_vrproject
    (:Is%20Valid
      (bind _output_get (Variables|Default|SetPlatform (Variables|/Game/BowAndMusket/Blueprints/GI_VRProject.GI_VRProject_C|GetPlatform _asgi_vrproject)))
      (return (Utilities|Select :Index _output_get :NewEnumerator0 (Variables|Default|GetPCMap) :NewEnumerator1 (Variables|Default|GetMobileMap))))))