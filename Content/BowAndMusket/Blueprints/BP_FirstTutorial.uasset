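; BP_FirstTutorial is a Blueprint that drives the tutorial messages for the player's first rotation and first teleport.
; On BeginPlay it takes the user widget from its Widget component, casts it to WB_Tutorial, stores it and passes itself to the widget.
; The FirstRotate and FirstTeleport events forward to the widget's matching message functions.
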(event EventBeginPlay
  (bind _aswb_tutorial (Utilities|Casting|CastToWB_Tutorial (UserInterface|GetUserWidgetObject (Variables|Default|GetWidget))))
  (bind _output_get (Variables|Default|SetTutorial%20Widget _aswb_tutorial))
  (Utilities|IsValid _output_get
    (:Is%20Valid
      (Default|GetTutorialObject _aswb_tutorial self))))

(event EventFirstRotate
  (Class|BPITutorial|FirstRotate(Message) (Variables|Default|GetTutorial%20Widget)))

(event EventFirstTeleport
  (Class|BPITutorial|FirstTeleport(Message) (Variables|Default|GetTutorial%20Widget)))

(fn ConstructionScript)