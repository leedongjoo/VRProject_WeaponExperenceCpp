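; BP_UMG_ExperenceMap is a Blueprint that hosts the WB_ChargingSequenceChecker UI through a widget component and relays charging sequence information to it.
; On BeginPlay it casts the component's user widget and caches the reference.
; The SendSequenceInfo and ResetVisibility events check that reference is valid, then forward to the matching calls on the widget.
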(event EventBeginPlay
  (bind _aswb_charging_sequence_checker (Utilities|Casting|CastToWB_ChargingSequenceChecker (UserInterface|GetUserWidgetObject (Variables|Default|GetWidget))))
  (Variables|Default|SetAs%20WB%20Charging%20Sequence%20Checker _aswb_charging_sequence_checker))

(event EventResetVisibility
  (bind _as_wb_charging_sequence_checker (Variables|Default|GetAs%20WB%20Charging%20Sequence%20Checker))
  (Utilities|IsValid _as_wb_charging_sequence_checker
    (:Is%20Valid
      (Default|ResetVisibility _as_wb_charging_sequence_checker))))

(event EventSendSequenceInfo
  (params (ChargingInfoToSendAtUI :type S%20Gun%20Charging%20Sequence%20Structure))
  (bind _as_wb_charging_sequence_checker (Variables|Default|GetAs%20WB%20Charging%20Sequence%20Checker))
  (Utilities|IsValid _as_wb_charging_sequence_checker
    (:Is%20Valid
      (Default|SendSequenceInfo _as_wb_charging_sequence_checker ChargingInfoToSendAtUI))))

(fn ConstructionScript)