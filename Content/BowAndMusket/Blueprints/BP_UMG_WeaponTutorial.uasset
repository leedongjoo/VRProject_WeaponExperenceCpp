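; BP_UMG_WeaponTutorial is an actor that hosts the WB_WeaponTutorial widget for the weapon tutorial through a widget component.
; On BeginPlay it casts the component's user widget and caches the reference.
; SendSequenceInfo passes charging info to that widget and ResetVisibility forwards a reset, each only while the cached reference is valid.
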(event EventBeginPlay
  (bind _aswb_weapon_tutorial (Utilities|Casting|CastToWB_WeaponTutorial (UserInterface|GetUserWidgetObject (Variables|Default|GetWidget))))
  (Variables|Default|SetAs%20WB%20Weapon%20Tutorial _aswb_weapon_tutorial))

(event EventResetVisibility
  (bind _as_wb_weapon_tutorial (Variables|Default|GetAs%20WB%20Weapon%20Tutorial))
  (Utilities|IsValid _as_wb_weapon_tutorial
    (:Is%20Valid
      (Default|ResetVisibility _as_wb_weapon_tutorial))))

(event EventSendSequenceInfo
  (params (ChargingInfoToSendAtUI :type S%20Gun%20Charging%20Sequence%20Structure))
  (bind _as_wb_weapon_tutorial (Variables|Default|GetAs%20WB%20Weapon%20Tutorial))
  (Utilities|IsValid _as_wb_weapon_tutorial
    (:Is%20Valid
      (Default|SendSequenceInfo _as_wb_weapon_tutorial ChargingInfoToSendAtUI))))

(fn ConstructionScript
  (|CallParentFunction))