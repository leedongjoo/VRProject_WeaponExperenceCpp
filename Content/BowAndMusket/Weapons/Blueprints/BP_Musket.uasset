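; Matchlock musket weapon child Blueprint with grip points and a staged manual reload.
; Loading events advance a charging-sequence struct through powder, ramming, bullet and paper wad, then priming powder in the opened pan, alongside match cord attachment.
; Trigger pulls animate the lock through Musket_AnimBP, remove the cord and, if pan powder exists, fire with recoil and reset.
; The construction script snaps grips, interaction triggers and charging widget to frame sockets.
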(event Custom|ReleaseTrigger
  ;[1 0.1701 0.2483] 머스킷 격발 - 방아쇠 컨트롤
  ;;[1 1 1] 트리거에서 손을 땔시
  (|CallParentFunction)
  (Variables|/Game/BowAndMusket/Weapons/Blueprints/Musket_AnimBP.Musket_AnimBP_C|SetPlayFireAnimation (Variables|Default|GetMusket%20Anim%20BP) false)
  (Variables|/Game/BowAndMusket/Weapons/Blueprints/Musket_AnimBP.Musket_AnimBP_C|SetTriggerRotationValue (Variables|Default|GetMusket%20Anim%20BP) "0, 0, 0"))

(event EventGetFire
  ;[1 0.3756 0.865] 조총의 장전 절차
  ;;[1 1 1] 세 번째 - 화약접시에 화약을 삽입하고 화승을 부착한다
  ;;;[1 1 1] 3. 화승을 어태치한다
  (if (not (Utilities|Struct|BreakS_GunChargingSequence (Variables|Default|GetGunChargingSequence)))
    (bind _returnvalue (Game|SpawnActorfromClass "/Game/BowAndMusket/Weapons/Blueprints/NotGuns/BP_Rope.BP_Rope_C" (Transformation|GetSocketTransform (Variables|Default|GetFrame) "FireTrigger" "RTS_World") "Undefined" 0 0))
    (bind _output_get (Variables|Default|SetAttachedRope _returnvalue))
    (Transformation|AttachComponentToComponent _output_get (Variables|Default|GetFrame) "FireTrigger" "SnapToTarget" "SnapToTarget" "SnapToTarget" true)
    (bind _structout (Utilities|Struct|SetmembersinS_GunChargingSequence (Variables|Default|GetGunChargingSequence) true))
    (CallFunction|SendSequence _structout)))

(event EventBeginPlay
  ;[1 1 1] BeginPlay - 애니메이션 블루프린트 레퍼런스 가저오기
  (|CallParentFunction)
  (bind _asmusket_anim_bp (Utilities|Casting|CastToMusket_AnimBP (Components|SkeletalMesh|GetAnimInstance (Variables|Default|GetFrame))))
  (Variables|Default|SetMusket%20Anim%20BP _asmusket_anim_bp)
  (CallFunction|SpawnGrabPositionObjects))

(event EventGetMud
  (bind _gunchargingsequence (Variables|Default|GetGunChargingSequence))
  ;[1 0.3756 0.865] 조총의 장전 절차
  ;;[1 1 1] 두 번째 - 총알을 삽입하고 종이로 총알을 밀봉한다
  (|CallParentFunction)
  ;;;[1 1 1] 총알 존재시
  (if (Utilities|Struct|BreakS_GunChargingSequence (Variables|Default|GetGunChargingSequence))
    ;;;[1 1 1] 종이가 존재하지 않는다면
    (if (not (Utilities|Struct|BreakS_GunChargingSequence _gunchargingsequence))
      (bind _structout (Utilities|Struct|SetmembersinS_GunChargingSequence _gunchargingsequence true)) ; 종이를 획득합니다
      (CallFunction|SendSequence _structout)
      (Variables|Default|SetFirstMudObjectDestroy true) ; 삽입 성공시 삭제 가능
      (CallFunction|RechargebyChargingSequence) ; 화약을 다진다
    )))

(event EventGetGunPowderCapPowder
  (bind _powderspawnloc (Variables|Default|GetPowderSpawnLoc))
  (bind _gunchargingsequence (Variables|Default|GetGunChargingSequence))
  (bind _returnvalue (Transformation|GetWorldTransform _powderspawnloc))
  ;[1 0.3756 0.865] 조총의 장전 절차
  ;;[1 1 1] 세 번째 - 화약접시에 화약을 삽입하고 화승을 부착한다
  ;;;[1 1 1] 2. 화약접시에 화약을 스폰한다
  (|CallParentFunction)
  (if (and (Utilities|Struct|BreakS_GunChargingSequence _gunchargingsequence) (Utilities|Struct|BreakS_GunChargingSequence _gunchargingsequence))
    (if (not (Utilities|Struct|BreakS_GunChargingSequence (Variables|Default|GetGunChargingSequence)))
      (bind _returnvalue_2 (Game|SpawnActorfromClass "/Game/BowAndMusket/Weapons/Blueprints/NotGuns/BP_GunPowder.BP_GunPowder_C" (Math|Transform|MakeTransform (.location _returnvalue) (.rotation _returnvalue) "1,1,1") "Undefined" 0 0))
      (Variables|Default|SetPowderCapPowderDestroy true)
      (bind _output_get (Variables|Default|SetAttachedPowder _returnvalue_2))
      (Transformation|AttachComponentToComponent _output_get _powderspawnloc "None" "SnapToTarget" "SnapToTarget" "SnapToTarget" true)
      (bind _structout (Utilities|Struct|SetmembersinS_GunChargingSequence (Variables|Default|GetGunChargingSequence) true))
      (CallFunction|SendSequence _structout)
      (CallFunction|FireTriggerCollisionToggle "QueryOnly") ; 파이어 트리거 콜리전 활성화
    )))

(event EventGetGunPowder
  (bind _gunchargingsequence (Variables|Default|GetGunChargingSequence))
  ;[1 0.3756 0.865] 조총의 장전 절차
  ;;[1 1 1] 첫 번째 - 총신을 세척하고 총신에 화약을 삽입한다
  (|CallParentFunction)
  ;;;[1 1 1] 화약 획득 상태라면
  (if (Utilities|Struct|BreakS_GunChargingSequence _gunchargingsequence)
    (if (not (Utilities|Struct|BreakS_GunChargingSequence _gunchargingsequence))
      (CallFunction|RechargebyChargingSequence) ; 화약을 다진다
    )))

(event EventGetBullet
  (bind _gunchargingsequence (Variables|Default|GetGunChargingSequence))
  ;[1 0.3756 0.865] 조총의 장전 절차
  ;;[1 1 1] 두 번째 - 총알을 삽입하고 종이로 총알을 밀봉한다
  (|CallParentFunction)
  (if (Utilities|Struct|BreakS_GunChargingSequence _gunchargingsequence) ; 2번째 차징 완료시 (순서에 따라)
    ;;;[1 1 1] 총알 존재X, 3번째 차징 완료되지 않았을 때
    (if (not (and (Utilities|Struct|BreakS_GunChargingSequence _gunchargingsequence) (Utilities|Struct|BreakS_GunChargingSequence _gunchargingsequence)))
      (bind _structout (Utilities|Struct|SetmembersinS_GunChargingSequence _gunchargingsequence true)) ; 총알을 획득합니다
      (CallFunction|SendSequence _structout))))

(event EventDeleteFire
  (bind _attachedrope (Variables|Default|GetAttachedRope))
  ;[1 0.1701 0.2483] 머스킷 격발 - 방아쇠 컨트롤
  ;;[1 1 1] 화승을 디스트로이한다
  (|CallParentFunction)
  (Utilities|IsValid _attachedrope
    (:Is%20Valid
      (Actor|DestroyActor _attachedrope)
      (Utilities|Struct|SetmembersinS_GunChargingSequence (Variables|Default|GetGunChargingSequence) false))))

(event EventUpdateChargingSequence
  ;[1 0.3756 0.865] 조총의 장전 절차
  (switch int (Variables|Default|GetChargingNumberCount) ; 차징 횟수에 따라 순서 구별
    (:1
      ;;[1 1 1] 첫 번째 - 총신을 세척하고 총신에 화약을 삽입한다
      (bind _structout (Utilities|Struct|SetmembersinS_GunChargingSequence (Variables|Default|GetGunChargingSequence) true))
      (CallFunction|SendSequence _structout))
    (:2
      ;;[1 1 1] 두 번째 - 총알을 삽입하고 종이로 총알을 밀봉한다
      (bind _structout_2 (Utilities|Struct|SetmembersinS_GunChargingSequence (Variables|Default|GetGunChargingSequence) true)) ; 화약 다지기 완료
      (CallFunction|SendSequence _structout_2))
    (:3
      ;;[1 1 1] 세 번째 - 화약접시에 화약을 삽입하고 화승을 부착한다
      (bind _structout_3 (Utilities|Struct|SetmembersinS_GunChargingSequence (Variables|Default|GetGunChargingSequence) true)) ; 최종 장전 완료
      (CallFunction|SendSequence _structout_3))))

(event EventRotatePowderCap
  (bind _gunchargingsequence (Variables|Default|GetGunChargingSequence))
  ;[1 0.3756 0.865] 조총의 장전 절차
  ;;[1 1 1] 세 번째 - 화약접시에 화약을 삽입하고 화승을 부착한다
  ;;;[1 1 1] 1. 화약접시를 연다
  (Utilities|FlowControl|FlipFlop
    (:A
      (Variables|/Game/BowAndMusket/Weapons/Blueprints/Musket_AnimBP.Musket_AnimBP_C|Set%20FirecapRotationValue (Variables|Default|GetMusket%20Anim%20BP) "0,-90.000000, 0")
      (Utilities|Struct|SetmembersinS_GunChargingSequence _gunchargingsequence true))
    (:B
      (Variables|/Game/BowAndMusket/Weapons/Blueprints/Musket_AnimBP.Musket_AnimBP_C|Set%20FirecapRotationValue (Variables|Default|GetMusket%20Anim%20BP) "0, 0, 0")
      (Utilities|Struct|SetmembersinS_GunChargingSequence _gunchargingsequence false))))

(event EventSpawnGrabPositionObjects
  ;[0.4115 1 0.2559] 스폰된 그랩 위치를 알려주는 오브젝트 위치에 따라 크기 변경
)

(event EventPulltheTrigger
  (bind _musket_anim_bp (Variables|Default|GetMusket%20Anim%20BP))
  (bind _attachedpowder (Variables|Default|GetAttachedPowder))
  ;[1 0.1701 0.2483] 머스킷 격발 - 방아쇠 컨트롤
  (|CallParentFunction)
  (if (not (Variables|Default|GetIsReloadingMode)) ; 장전 상태가 아니여야 함
    ;;[1 1 1] 격발시 용두가 내려가는 애니메이션 재생
    (Variables|/Game/BowAndMusket/Weapons/Blueprints/Musket_AnimBP.Musket_AnimBP_C|SetPlayFireAnimation _musket_anim_bp true)
    (Variables|/Game/BowAndMusket/Weapons/Blueprints/Musket_AnimBP.Musket_AnimBP_C|SetTriggerRotationValue _musket_anim_bp "0, 0,40.000000")
    (Utilities|FlowControl|Delay 0.2) ; 애니메이션 재생 시간
    (CallFunction|DeleteFire) ; 화승 없애기
    (Utilities|IsValid _attachedpowder ; 화약접시의 화약 존재
      (:Is%20Valid
        (Actor|DestroyActor _attachedpowder) ; 총에 부착된 화약 없애기
        (CallFunction|SpawnEmitterandRecoil) ; 총알 발사(총알 여부에 따라 달라짐)
        (CallFunction|RespawnAll) ; 화약 리스폰
      ))))

(fn ConstructionScript
  (bind _frame (Variables|Default|GetFrame))
  (bind _frame_2 (Variables|Default|GetFrame))
  (bind _frame_3 (Variables|Default|GetFrame))
  (bind _frame_4 (Variables|Default|GetFrame))
  (bind _frame_5 (Variables|Default|GetFrame))
  (bind _returnvalue (Transformation|GetSocketTransform _frame_3 "TwoHandGrip" "RTS_World"))
  (bind _returnvalue_2 (Transformation|GetSocketTransform _frame_2 "PowderCap" "RTS_World"))
  (bind _returnvalue_3 (Transformation|GetSocketTransform _frame_4 "OneHandGrip" "RTS_World"))
  (bind _returnvalue_4 (Transformation|GetSocketTransform _frame "FireTrigger" "RTS_World"))
  (bind _returnvalue_5 (Transformation|GetSocketTransform _frame_5 "FirePos" "RTS_World"))
  (bind (_location _rotation) (Math|Transform|BreakTransform _returnvalue_2))
  (bind (_location_2 _rotation_2) (Math|Transform|BreakTransform _returnvalue_5))
  (bind (_location_3 _rotation_3) (Math|Transform|BreakTransform _returnvalue_4))
  (bind (_location_4 _rotation_4) (Math|Transform|BreakTransform _returnvalue))
  (bind (_location_5 _rotation_5) (Math|Transform|BreakTransform _returnvalue_3))
  (|CallParentFunction)
  (Transformation|AttachComponentToComponent (Variables|Default|GetPowderSpawnLoc) (Variables|Default|GetTriggerBoxParent) "None" "KeepRelative" "KeepRelative" "KeepRelative" true)
  (Transformation|SetWorldLocationAndRotation (Variables|Default|Get2ndGrab) _location_4 _rotation_4 false false)
  (Transformation|SetWorldLocationAndRotation (Variables|Default|Get1ndGrab) _location_5 _rotation_5 false false)
  (Transformation|SetWorldLocationAndRotation (Variables|Default|GetFireTrigger) _location_3 _rotation_3 false false)
  (Transformation|SetWorldLocationAndRotation (Variables|Default|GetPowderTrigger) _location _rotation false false)
  (Transformation|SetWorldLocationAndRotation (Variables|Default|GetChargingTrigger) _location_2 _rotation_2 false false)
  (Transformation|SetWorldLocationAndRotation (Variables|Default|GetChargingBarWidget) (.Location (Math|Transform|BreakTransform (Transformation|GetSocketTransform (Variables|Default|GetFrame) "FirePos" "RTS_World"))) "90.000000, 0,0.000000" false false))