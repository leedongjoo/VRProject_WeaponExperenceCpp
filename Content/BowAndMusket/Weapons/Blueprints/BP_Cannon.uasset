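; BP_Cannon is a child weapon Blueprint for a muzzle-loaded cannon, fired by a fuse after a staged manual loading sequence.
; Parent weapon events and the charge count advance GunChargingSequence through powder, mud wad, packing and projectile, which spawns attached at the muzzle and enables the fire trigger.
; GetFire attaches BP_Fire at the rope socket, then removes it and fires with recoil after a delay.
; The construction script snaps grips, triggers and charging widget to Frame sockets.
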(event EventBeginPlay
  ;[1 1 1] BeginPlay
  (|CallParentFunction)
  (CallFunction|SpawnGrabPositionObjects))

(event EventDeleteFire
  (bind _attachedfire (Variables|Default|GetAttachedFire))
  ;[1 1 1] 불 삭제
  (|CallParentFunction)
  (Utilities|IsValid _attachedfire
    (:Is%20Valid
      (Actor|DestroyActor _attachedfire)
      (Variables|Default|SetFireAttachable true))))

(event EventSpawnGrabPositionObjects
  ;[1 1 1] 스폰된 그랩 포지션 오브젝트 무기에 맞게 크기 변경
)

(event EventGetGunPowder
  ;[1 1 1] 비격진천뢰 장전 절차
  ;;[1 0 0.03529] 첫 번째(공통) - 총구를 세척하고 총구에 화약을 삽입, 토격으로 화약을 밀봉한다
  (|CallParentFunction))

(event EventGetFire
  (bind _frame (Variables|Default|GetFrame))
  (bind _returnvalue (Transformation|GetSocketTransform _frame "FireRopePos" "RTS_World"))
  ;[1 1 1] 불 스폰 후 어태치
  (if (Variables|Default|GetFireAttachable)
    (bind _returnvalue_2 (Game|SpawnActorfromClass "/Game/BowAndMusket/Weapons/Blueprints/NotGuns/BP_Fire.BP_Fire_C" (Math|Transform|MakeTransform (.location _returnvalue) (.rotation _returnvalue) (.scale _returnvalue)) "Undefined" 0 0))
    (bind _output_get (Variables|Default|SetAttachedFire _returnvalue_2))
    (Transformation|AttachComponentToComponent _output_get (Variables|Default|GetFrame) "FireRopePos" "SnapToTarget" "SnapToTarget" "KeepWorld" true)
    (Variables|Default|SetFireAttachable false)
    (Utilities|IsValid (Variables|Default|GetAttachedFire) ; 불이 부착 시
      (:Is%20Valid
        (bind _structout (Utilities|Struct|SetmembersinS_GunChargingSequence (Variables|Default|GetGunChargingSequence) true)) ; 최종 장전 완료
        (CallFunction|SendSequence _structout)
        ;[1 1 1] 화약이 있음 - 그대로 발사
        (Utilities|FlowControl|Delay 3.0) ; 3초 뒤
        (CallFunction|DeleteFire)
        (CallFunction|SpawnEmitterandRecoil) ; 총알 발사
      ))))

(event EventGetBullet
  (bind _gunchargingsequence (Variables|Default|GetGunChargingSequence))
  ;[1 1 1] 비격진천뢰 장전 절차
  ;;[1 0 0.03529] 두 번째 - 총알 삽입, 불 부착 및 격발한다
  (|CallParentFunction)
  (if (Utilities|Struct|BreakS_GunChargingSequence _gunchargingsequence) ; 2번째 차징 완료시(순서에 따라)
    (if (not (Utilities|Struct|BreakS_GunChargingSequence _gunchargingsequence)) ; 총알 존재 X 시
      (bind _spawnedprojectile (CallFunction|BulletSpawn)) ; 총알을 총구에 스폰한다
      (bind _structout (Utilities|Struct|SetmembersinS_GunChargingSequence _gunchargingsequence true)) ; 총알을 획득합니다
      (CallFunction|SendSequence _structout)
      (bind _output_get (Variables|Default|SetSpawned%20Projectile _spawnedprojectile))
      (Transformation|AttachComponentToComponent _output_get (Variables|Default|GetFrame) "FirePos" "SnapToTarget" "SnapToTarget" "SnapToTarget" false)
      (Utilities|Struct|SetmembersinS_GunChargingSequence (Variables|Default|GetGunChargingSequence) true) ; 최종 장전 완료
      (CallFunction|FireTriggerCollisionToggle "QueryOnly") ; 파이어 트리거 콜리전 활성화
    )))

(event EventUpdateChargingSequence
  ;[1 1 1] 비격진천뢰 장전 절차
  (Utilities|FlowControl|Sequence
    (:then_0
      (switch int (Variables|Default|GetChargingNumberCount) ; 차징 횟수에 따라 순서 구별
        (:1
          ;;[1 0 0.03529] 첫 번째(공통) - 총구를 세척하고 총구에 화약을 삽입, 토격으로 화약을 밀봉한다
          (bind _structout (Utilities|Struct|SetmembersinS_GunChargingSequence (Variables|Default|GetGunChargingSequence) true))
          (CallFunction|SendSequence _structout))
        (:2
          ;;[1 0 0.03529] 두 번째 - 총알 삽입, 불 부착 및 격발한다
          (bind _structout_2 (Utilities|Struct|SetmembersinS_GunChargingSequence (Variables|Default|GetGunChargingSequence) true)) ; 화약 다지기 완료
          (CallFunction|SendSequence _structout_2))))))

(event EventGetMud
  ;[1 1 1] 비격진천뢰 장전 절차
  ;;[1 0 0.03529] 첫 번째(공통) - 총구를 세척하고 총구에 화약을 삽입, 토격으로 화약을 밀봉한다
  ;;;[1 1 1] 첫 번째 순서에 따라
  (|CallParentFunction)
  (if (and (Utilities|Struct|BreakS_GunChargingSequence (Variables|Default|GetGunChargingSequence)) (not (Utilities|Struct|BreakS_GunChargingSequence (Variables|Default|GetGunChargingSequence))))
    (if (Utilities|Struct|BreakS_GunChargingSequence (Variables|Default|GetGunChargingSequence)) ; 화약이 존재한다면
      (if (not (Utilities|Struct|BreakS_GunChargingSequence (Variables|Default|GetGunChargingSequence))) ; 토격이 존재하지 않는다면
        (bind _structout (Utilities|Struct|SetmembersinS_GunChargingSequence (Variables|Default|GetGunChargingSequence) true)) ; 토격 삽입
        (CallFunction|SendSequence _structout)
        (Variables|Default|SetFirstMudObjectDestroy true) ; 삽입 성공시 삭제 가능
        (CallFunction|RechargebyChargingSequence) ; 장전 상태 초기화
      ))))

(fn ConstructionScript
  (bind _frame (Variables|Default|GetFrame))
  (bind _frame_2 (Variables|Default|GetFrame))
  (bind _frame_3 (Variables|Default|GetFrame))
  (bind _frame_4 (Variables|Default|GetFrame))
  (bind _frame_5 (Variables|Default|GetFrame))
  (bind _returnvalue (Transformation|GetSocketTransform _frame_4 "FireTrigger" "RTS_World"))
  (bind _returnvalue_2 (Transformation|GetSocketTransform _frame_3 "TwoHandGrip" "RTS_World"))
  (bind _returnvalue_3 (Transformation|GetSocketTransform _frame_2 "ReloadPos" "RTS_World"))
  (bind _returnvalue_4 (Transformation|GetSocketTransform _frame_5 "ReloadPos" "RTS_World"))
  (bind _returnvalue_5 (Transformation|GetSocketTransform _frame "OneHandGrip" "RTS_World"))
  (bind (_location _rotation) (Math|Transform|BreakTransform _returnvalue))
  (bind (_location_2 _rotation_2) (Math|Transform|BreakTransform _returnvalue_3))
  (bind (_location_3 _rotation_3) (Math|Transform|BreakTransform _returnvalue_5))
  (bind (_location_4 _rotation_4) (Math|Transform|BreakTransform _returnvalue_2))
  (bind (_location_5 _rotation_5) (Math|Transform|BreakTransform _returnvalue_4))
  (|CallParentFunction)
  (Utilities|FlowControl|Sequence
    (:then_0
      (Transformation|AttachComponentToComponent (Variables|Default|GetRope) (Variables|Default|GetTriggerBoxParent) "None" "KeepRelative" "KeepRelative" "KeepRelative" true))
    (:then_1
      (Transformation|SetWorldLocationAndRotation (Variables|Default|Get1ndGrab) _location_3 _rotation_3 false false)
      (Transformation|SetWorldLocationAndRotation (Variables|Default|Get2ndGrab) _location_4 _rotation_4 false false)
      (Transformation|SetWorldLocationAndRotation (Variables|Default|GetFireTrigger) _location _rotation false false)
      (Transformation|SetWorldLocationAndRotation (Variables|Default|GetChargingTrigger) _location_5 _rotation_5 false false)
      (Transformation|SetWorldLocationAndRotation (Variables|Default|GetPowderTrigger) _location_2 _rotation_2 false false)
      (Transformation|SetWorldLocationAndRotation (Variables|Default|GetChargingBarWidget) (.Location (Math|Transform|BreakTransform (Transformation|GetSocketTransform (Variables|Default|GetFrame) "FirePos" "RTS_World"))) "90.000000, 0, 0" false false))))