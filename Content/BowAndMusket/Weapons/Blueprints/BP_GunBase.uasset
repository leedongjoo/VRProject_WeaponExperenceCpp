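; Base Blueprint for hand-held black-powder guns (Seung Jar Gun, Musket, Cannon Ball) with haptics and staged reloading, leaving weapon-specific steps to children.
; Socket-placed markers show grab and loading points, with visibility following trigger collision as general and reload modes toggle.
; A timeline-driven pole performs charging, and loading progress goes to UI actors.
; Firing spawns a type-specific projectile, pulses a physics thruster for recoil, then resets loading and respawns supplies.
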(event Custom|GetFire
  ;[1 0.2849 0.5455] 코어 - 오브젝트 컨트롤
  ;;[1 1 1] 기타 이벤트 / 차일드에서 구현
)

(event Custom|GetGunPowder
  (bind _gunchargingsequence (Variables|GunChargingOrderFlags|GetGunChargingSequence))
  ;[1 0.2849 0.5455] 코어 - 오브젝트 컨트롤
  ;;[1 1 1] 총구 화약 획득 / 차일드에서 구현
  (Variables|Default|SetFiringPowderObjectDestroy false) ; 변수 초기화
  (if (and (.InitialChargingComplete (Utilities|Struct|BreakS_GunChargingSequence (Variables|GunChargingOrderFlags|GetGunChargingSequence))) (not (.2ndFPowderChargingComplete (Utilities|Struct|BreakS_GunChargingSequence (Variables|GunChargingOrderFlags|GetGunChargingSequence))))) ; 해당 순서에만 발동
    (if (not (.HasFiringPowder (Utilities|Struct|BreakS_GunChargingSequence _gunchargingsequence))) ; 현재 화약 가지고 있지 않다면
      (bind _structout (Utilities|Struct|SetmembersinS_GunChargingSequence _gunchargingsequence true)) ; 화약을 획득합니다
      (Variables|Default|SetFiringPowderObjectDestroy true)
      (CallFunction|SendSequence _structout))))

(event Custom|RechargeByChargingSequence
  ;[1 0.6305 0.8684] 코어 - 장전 기능
  ;;[0.2246 1 0.2011] 장전상태 리셋(관련 변수 초기화)
  (Variables|Default|SetAllowPoleMovement true)
  (Variables|Default|SetChargingTimes 0.0))

(event Custom|Charging%20Trigger%20Collision%20Toggle
  (params (New%20CollisionType :type ECollisionEnabled%20Enum :default "NoCollision"))
  (bind _chargingtrigger (Variables|Default|GetChargingTrigger))
  ;[0.454 1 0.9701] 콜리전 토글
  (Utilities|IsValid _chargingtrigger
    (:Is%20Valid
      (Collision|SetCollisionEnabled _chargingtrigger New%20CollisionType)
      (CallFunction|SetPositionObjectVisibility true (Variables|PositionObject|GetFirePosObj) _chargingtrigger))))

(event Custom|SpawnGrabPositionObjects
  (bind _frame (Variables|Default|GetFrame))
  (bind _frame_2 (Variables|Default|GetFrame))
  (bind _frame_3 (Variables|Default|GetFrame))
  (bind _frame_4 (Variables|Default|GetFrame))
  (bind _frame_5 (Variables|Default|GetFrame))
  ;[1 0.8353 0.3059] 상호작용할 컴포넌트 위치를 알려주는 오브젝트들을 스폰한다
  (Utilities|FlowControl|Sequence
    (:then_0
      (if (Transformation|DoesSocketExist _frame_3 "OneHandGrip")
        (Variables|Default|SetOneHandGripTransform (Transformation|GetSocketTransform _frame_3 "OneHandGrip" "RTS_World"))
        (bind _returnvalue (Game|SpawnActorfromClass "/Game/BowAndMusket/Weapons/Blueprints/NotGuns/BP_WeaponGrabPosition.BP_WeaponGrabPosition_C" (Math|Transform|MakeTransform (.location (Variables|Default|GetOneHandGripTransform)) (.rotation (Variables|Default|GetOneHandGripTransform)) "1,1,1") "Undefined" 0 0))
        (Utilities|IsValid _returnvalue
          (:Is%20Valid
            (bind _output_get (Variables|PositionObject|Set1ndGrabPosObj _returnvalue))
            (Transformation|AttachComponentToComponent _output_get (Variables|Default|GetFrame) "OneHandGrip" "SnapToTarget" "SnapToTarget" "KeepWorld" true)))))
    (:then_1
      (switch Utilities|FlowControl|Switch|SwitchonE_Weapons (Variables|WeaponType|GetWeaponType) ; 비격진천뢰는 FireTrigger에 오브젝트가 스폰되지 않음
        (:NewEnumerator0
          _)
        (:NewEnumerator2
          _))
      (if (Transformation|DoesSocketExist _frame_4 "FireTrigger")
        (Variables|Default|SetRopePositionTransform (Transformation|GetSocketTransform _frame_4 "FireTrigger" "RTS_World"))
        (bind _returnvalue_2 (Game|SpawnActorfromClass "/Game/BowAndMusket/Weapons/Blueprints/NotGuns/BP_WeaponGrabPosition.BP_WeaponGrabPosition_C" (Math|Transform|MakeTransform (.location (Variables|Default|GetRopePositionTransform)) (.rotation (Variables|Default|GetRopePositionTransform)) "1,1,1") "Undefined" 0 0))
        (Utilities|IsValid _returnvalue_2
          (:Is%20Valid
            (bind _output_get_2 (Variables|PositionObject|SetRopePosObj _returnvalue_2))
            (Transformation|AttachComponentToComponent _output_get_2 (Variables|Default|GetFrame) "FireTrigger" "SnapToTarget" "SnapToTarget" "KeepWorld" true)))))
    (:then_2
      (if (Transformation|DoesSocketExist _frame_5 "FirePos")
        (Variables|Default|SetFirePosTransform (Transformation|GetSocketTransform _frame_5 "FirePos" "RTS_World"))
        (bind _returnvalue_3 (Game|SpawnActorfromClass "/Game/BowAndMusket/Weapons/Blueprints/NotGuns/BP_WeaponGrabPosition.BP_WeaponGrabPosition_C" (Math|Transform|MakeTransform (.location (Variables|Default|GetFirePosTransform)) (.rotation (Variables|Default|GetFirePosTransform)) "1,1,1") "Undefined" 0 0))
        (Utilities|IsValid _returnvalue_3
          (:Is%20Valid
            (bind _output_get_3 (Variables|PositionObject|SetFirePosObj _returnvalue_3))
            (Transformation|AttachComponentToComponent _output_get_3 (Variables|Default|GetFrame) "FirePos" "SnapToTarget" "SnapToTarget" "KeepWorld" true)))))
    (:then_3
      (if (Transformation|DoesSocketExist _frame_2 "TwoHandGrip")
        (Variables|Default|SetTwoHandGripTransform (Transformation|GetSocketTransform _frame_2 "TwoHandGrip" "RTS_World"))
        (bind _returnvalue_4 (Game|SpawnActorfromClass "/Game/BowAndMusket/Weapons/Blueprints/NotGuns/BP_WeaponGrabPosition.BP_WeaponGrabPosition_C" (Math|Transform|MakeTransform (.location (Variables|Default|GetTwoHandGripTransform)) (.rotation (Variables|Default|GetTwoHandGripTransform)) "1,1,1") "Undefined" 0 0))
        (Utilities|IsValid _returnvalue_4
          (:Is%20Valid
            (bind _output_get_4 (Variables|PositionObject|SetTwoHandGripPosObj _returnvalue_4))
            (Transformation|AttachComponentToComponent _output_get_4 (Variables|Default|GetFrame) "TwoHandGrip" "SnapToTarget" "SnapToTarget" "KeepWorld" true)))))
    (:then_4
      (if (Transformation|DoesSocketExist _frame "PowderCap")
        (Variables|Default|SetPowderCapTransform (Transformation|GetSocketTransform _frame "PowderCap" "RTS_World"))
        (bind _returnvalue_5 (Game|SpawnActorfromClass "/Game/BowAndMusket/Weapons/Blueprints/NotGuns/BP_WeaponGrabPosition.BP_WeaponGrabPosition_C" (Math|Transform|MakeTransform (.location (Variables|Default|GetPowderCapTransform)) (.rotation (Variables|Default|GetPowderCapTransform)) "1,1,1") "Undefined" 0 0))
        (Utilities|IsValid _returnvalue_5
          (:Is%20Valid
            (bind _output_get_5 (Variables|PositionObject|SetPowderCapPosObj _returnvalue_5))
            (Transformation|AttachComponentToComponent _output_get_5 (Variables|Default|GetFrame) "PowderCap" "SnapToTarget" "SnapToTarget" "KeepWorld" true)))))))

(event Custom|Fire%20Trigger%20Collision%20Toggle
  (params (New%20CollisionType :type ECollisionEnabled%20Enum :default "NoCollision"))
  (bind _firetrigger (Variables|Default|GetFireTrigger))
  ;[0.454 1 0.9701] 콜리전 토글
  (Utilities|IsValid _firetrigger
    (:Is%20Valid
      (Collision|SetCollisionEnabled _firetrigger New%20CollisionType)
      (CallFunction|SetPositionObjectVisibility true (Variables|PositionObject|GetRopePosObj) _firetrigger))))

(event Custom|1nd%20Grab%20Collision%20Toggle
  (params (New%20CollisionType :type ECollisionEnabled%20Enum :default "NoCollision"))
  (bind _1ndgrab (Variables|Default|Get1ndGrab))
  ;[0.454 1 0.9701] 콜리전 토글
  (Utilities|IsValid _1ndgrab
    (:Is%20Valid
      (Collision|SetCollisionEnabled _1ndgrab New%20CollisionType)
      (CallFunction|SetPositionObjectVisibility true (Variables|PositionObject|Get1ndGrabPosObj) _1ndgrab))))

(event Custom|ResetPositionObjectsVisibility
  (bind _1ndgrabposobj (Variables|PositionObject|Get1ndGrabPosObj))
  (bind _ropeposobj (Variables|PositionObject|GetRopePosObj))
  (bind _fireposobj (Variables|PositionObject|GetFirePosObj))
  (bind _twohandgripposobj (Variables|PositionObject|GetTwoHandGripPosObj))
  (bind _powdercapposobj (Variables|PositionObject|GetPowderCapPosObj))
  ;[1 0.8353 0.3059] 그랩 포지션 오브젝트 비저빌리티 온
  (Utilities|FlowControl|Sequence
    (:then_0
      (Utilities|IsValid _1ndgrabposobj
        (:Is%20Valid
          (Rendering|SetVisibility (Variables|/Game/BowAndMusket/Weapons/Blueprints/NotGuns/BP_WeaponGrabPosition.BP_WeaponGrabPosition_C|GetSphere _1ndgrabposobj) true false))))
    (:then_1
      (Utilities|IsValid _ropeposobj
        (:Is%20Valid
          (Rendering|SetVisibility (Variables|/Game/BowAndMusket/Weapons/Blueprints/NotGuns/BP_WeaponGrabPosition.BP_WeaponGrabPosition_C|GetSphere _ropeposobj) true false))))
    (:then_2
      (Utilities|IsValid _fireposobj
        (:Is%20Valid
          (Rendering|SetVisibility (Variables|/Game/BowAndMusket/Weapons/Blueprints/NotGuns/BP_WeaponGrabPosition.BP_WeaponGrabPosition_C|GetSphere _fireposobj) true false))))
    (:then_3
      (Utilities|IsValid _twohandgripposobj
        (:Is%20Valid
          (Rendering|SetVisibility (Variables|/Game/BowAndMusket/Weapons/Blueprints/NotGuns/BP_WeaponGrabPosition.BP_WeaponGrabPosition_C|GetSphere _twohandgripposobj) true false))))
    (:then_4
      (Utilities|IsValid _powdercapposobj
        (:Is%20Valid
          (Rendering|SetVisibility (Variables|/Game/BowAndMusket/Weapons/Blueprints/NotGuns/BP_WeaponGrabPosition.BP_WeaponGrabPosition_C|GetSphere _powdercapposobj) true false))))))

(event Custom|Switch%20to%20Charging%20Mode
  ;[1 0.6394 0.992] 모드 체인지
  ;;[1 1 1] 컴포넌트 콜리전 세팅 - 장전 모드
  (Variables|Default|SetIsReloadingMode true)
  (Utilities|FlowControl|Sequence
    (:then_0
      (CallFunction|DeleteFire) ; 정전 모드로 변경 시 불 삭제
      (CallFunction|1ndGrabCollisionToggle "NoCollision") ; 장전 모드 - 그랩 콜리전 비활성화
      (CallFunction|ChargingTriggerCollisionToggle "QueryOnly") ; 장전 모드 - 장전 트리거 콜리전 활성화
      (Rendering|SetVisibility (Variables|Default|GetChargingBarWidget) true false) ; 장전 위젯 보이게함
    )
    (:then_1
      (Utilities|FlowControl|DoOnce false
        (:Completed
          (bind _structout (Utilities|Struct|SetmembersinS_GunChargingSequence (Variables|GunChargingOrderFlags|GetGunChargingSequence) true))
          (CallFunction|SendSequence _structout) ; UI로 전송
        )))))

(event Custom|2nd%20Grab%20Collision%20Toggle
  (params (New%20CollisionType :type ECollisionEnabled%20Enum :default "NoCollision"))
  (bind _2ndgrab (Variables|Default|Get2ndGrab))
  ;[0.454 1 0.9701] 콜리전 토글
  (Utilities|IsValid _2ndgrab
    (:Is%20Valid
      (Collision|SetCollisionEnabled _2ndgrab New%20CollisionType)
      (CallFunction|SetPositionObjectVisibility true (Variables|PositionObject|GetTwoHandGripPosObj) _2ndgrab))))

(event Custom|SetPositionObjectVisibility
  (params (VisibilityActivate :type Boolean) (PositionObject :type BP%20Weapon%20Grab%20Position%20Object%20Reference) (WeaponTriggerComponent :type Box%20Component%20Object%20Reference))
  (bind _sphere (Variables|/Game/BowAndMusket/Weapons/Blueprints/NotGuns/BP_WeaponGrabPosition.BP_WeaponGrabPosition_C|GetSphere PositionObject))
  ;[1 0.8353 0.3059] 그랩 포지션 오브젝트 비저빌리티 토글
  (Utilities|FlowControl|Sequence
    (:then_0
      (Utilities|IsValid PositionObject
        (:Is%20Valid
          (Rendering|SetVisibility (Variables|/Game/BowAndMusket/Weapons/Blueprints/NotGuns/BP_WeaponGrabPosition.BP_WeaponGrabPosition_C|GetSphere PositionObject) VisibilityActivate false) ; 비저빌리티 비활성화 / 활성화
        )))
    (:then_1
      (if VisibilityActivate
        (Utilities|IsValid WeaponTriggerComponent
          (:Is%20Valid
            (switch Utilities|FlowControl|Switch|SwitchonECollisionEnabled (Collision|GetCollisionEnabled WeaponTriggerComponent)
              (:NoCollision
                (Utilities|IsValid PositionObject
                  (:Is%20Valid
                    (Rendering|SetVisibility _sphere false false))))
              (:QueryOnly
                (Utilities|IsValid PositionObject :!label _label
                  (:Is%20Valid
                    (Rendering|SetVisibility _sphere true false))))
              (:QueryAndPhysics
                (goto _label)))))))))

(event Custom|Switch%20to%20Generel%20Mode
  ;[1 0.6394 0.992] 모드 체인지
  (Variables|Default|SetIsReloadingMode false)
  (Rendering|SetVisibility (Variables|Default|GetChargingBarWidget) false false) ; 장전 위젯 안보이게 함
  ;;[1 1 1] 컴포넌트 콜리전 세팅 - 일반 모드
  (CallFunction|1ndGrabCollisionToggle "QueryOnly") ; 1nd Grab 트리거 콜리전 활성화
  (CallFunction|ChargingTriggerCollisionToggle "NoCollision") ; 장전 트리거 콜리전 비활성화
)

(event Custom|SpawnEmitterandRecoil
  (bind _physicsthruster (Variables|Default|GetPhysicsThruster))
  (bind _frame (Variables|Default|GetFrame))
  (bind _returnvalue (Transformation|GetSocketTransform _frame "FirePos" "RTS_World"))
  (bind (_location _rotation) (Math|Transform|BreakTransform _returnvalue))
  ;[1 0 0.02424] 이미터 스폰, 반동 추가
  (Audio|PlaySound2D (Variables|GunSettings|GetShootingGunSound) 1.0 (Math|Random|RandomFloatinRange 0.9 1.1) 0.0 0 0)
  (Variables|Default|SetWeaponFirePosition _returnvalue)
  (Effects|SpawnEmitteratLocation (Variables|GunSettings|GetGunShotEmitter) _location _rotation) ; 총구 위치에 이미터 추가
  ;;[1 1 1] 총알이 있다면 총알 스폰 후 발사
  (bind _spawnedprojectile (CallFunction|BulletSpawn)) ; 이미 스폰된 총알이 있으면 없애고 총알을 스폰한다
  (CallFunction|ActivateSpawnedBullet _spawnedprojectile) ; 스폰한 총알을 발사한다
  (CallFunction|AfterFiring)
  ;;[1 1 1] 진동과 반동 추가
  (|RumbleController)
  (if (Physics|IsSimulatingPhysics (Variables|Default|GetFrame) "None")
    (Variables|/Script/Engine.PhysicsThrusterComponent|SetThrustStrength _physicsthruster (* (Variables|Default|GetInitialThrustStrength) (Variables|GunSettings|GetRecoilAmount) (select (Variables|Default|Get2HandendGrab) (Variables|GunSettings|Get2HandedRecoilMultiplier) 1.0)))
    (Components|Activation|Activate _physicsthruster true)
    (Utilities|FlowControl|RetriggerableDelay 0.1)
    (Components|Activation|Deactivate _physicsthruster)))

(event Custom|UpdateChargingSequence
  ;[1 0.6305 0.8684] 코어 - 장전 기능
)

(event Custom|Reset%20all%20Charging%20Seqence
  ;[1 0.6305 0.8684] 코어 - 장전 기능
  ;;[0.2246 1 0.2011] 장전상태 리셋(관련 변수 초기화)
  (Variables|Default|SetAllowPoleMovement true)
  (Variables|Default|SetChargingTimes 0.0)
  (Variables|GunChargingOrderFlags|SetChargingNumberCount 0)
  (Utilities|Struct|SetmembersinS_GunChargingSequence (Variables|GunChargingOrderFlags|GetGunChargingSequence) false false false false false false false false false)
  (for _array_element (Variables|Default|GetUIActors)
    (Utilities|IsValid _array_element
      (:Is%20Valid
        (Default|ResetVisibility _array_element)))))

(event Custom|Init%20Gun%20Components%20Collision
  ;[0.454 1 0.9701] 콜리전 토글
)

(event Custom|AfterFiring
  ;[1 0 0.02424] 이미터 스폰, 반동 추가
  (CallFunction|ResetAllChargingSeqence) ; 장전상태 리셋
  (CallFunction|FireTriggerCollisionToggle "NoCollision")
  (CallFunction|RespawnAll))

(event Custom|SendSequence
  (params (GunChargingSequence :type S%20Gun%20Charging%20Sequence%20Structure))
  ;[1 1 1] BeginPlay
  (for _array_element (Variables|Default|GetUIActors)
    (Utilities|IsValid _array_element
      (:Is%20Valid
        (Default|SendSequenceInfo _array_element GunChargingSequence)))))

(event Custom|GetMud
  ;[1 0.2849 0.5455] 코어 - 오브젝트 컨트롤
  ;;[1 1 1] 총알 획득 / 차일드에서 구현
  (Variables|Default|SetFirstMudObjectDestroy false) ; 변수 초기화
)

(event Custom|Pull%20The%20Trigger
  ;[1 0.2849 0.5455] 코어 - 오브젝트 컨트롤
  ;;[1 1 1] 기타 이벤트 / 차일드에서 구현
  ;;;[1 1 1] Musket 사용 이벤트
)

(event Custom|Get%20Gun%20PowderCap%20Powder
  ;[1 0.2849 0.5455] 코어 - 오브젝트 컨트롤
  ;;[1 1 1] 기타 이벤트 / 차일드에서 구현
  ;;;[1 1 1] Musket 사용 이벤트
  (Variables|Default|SetPowderCapPowderDestroy false))

(event Custom|Respawn%20All
  ;[1 0.2849 0.5455] 코어 - 오브젝트 컨트롤
  ;;[1 1 1] 총 다 쏘고 나서 화약과 토격을 리스폰한다
  (bind _outactors (Actor|GetAllActorsOfClass "/Game/BowAndMusket/Blueprints/BP_PhysicalObjectSpawner.BP_PhysicalObjectSpawner_C"))
  (for _array_element _outactors
    (Utilities|IsValid _array_element
      (:Is%20Valid
        (Default|RespawnAll _array_element)))))

(event Custom|RotatePowderCap
  ;[1 0.2849 0.5455] 코어 - 오브젝트 컨트롤
  ;;[1 1 1] 기타 이벤트 / 차일드에서 구현
  ;;;[1 1 1] Musket 사용 이벤트
)

(event Custom|GetBullet
  ;[1 0.2849 0.5455] 코어 - 오브젝트 컨트롤
  ;;[1 1 1] 총알 획득 / 차일드에서 구현
)

(event Custom|DeleteFire
  ;[1 0.2849 0.5455] 코어 - 오브젝트 컨트롤
  ;;[1 1 1] 기타 이벤트 / 차일드에서 구현
)

(event Custom|End%20Charging
  (bind _poleobject (Variables|Default|GetPoleObject))
  ;[1 0.6305 0.8684] 코어 - 장전 기능
  ;;[1 1 1] 손을 놓았을 때, 장전을 끝냄
  (if (Variables|GunChargingOrderFlags|GetIsCharging)
    (Variables|GunChargingOrderFlags|SetIsCharging false)
    (Variables|Default|SetChargingTimes -1.0)
    (Utilities|IsValid _poleobject
      (:Is%20Valid
        (Actor|DestroyActor _poleobject)))))

(event Custom|Powder%20Trigger%20Collision%20Toggle
  (params (NewCollisionType :type ECollisionEnabled%20Enum :default "NoCollision"))
  (bind _powdertrigger (Variables|Default|GetPowderTrigger))
  ;[0.454 1 0.9701] 콜리전 토글
  (Utilities|IsValid _powdertrigger
    (:Is%20Valid
      (Collision|SetCollisionEnabled _powdertrigger NewCollisionType)
      (CallFunction|SetPositionObjectVisibility true (Variables|PositionObject|GetPowderCapPosObj) _powdertrigger))))

(event Custom|Start%20Pole%20Movement
  (bind _chargingtimes (Variables|Default|GetChargingTimes))
  ;[1 0.6305 0.8684] 코어 - 장전 기능
  (if (Variables|Default|GetAllowPoleMovement) ; 차징 허용 여부
    ;;[1 1 1] 차징 중이 아닐때
    (if (not (Variables|GunChargingOrderFlags|GetIsCharging))
      (Variables|GunChargingOrderFlags|SetIsCharging true) ; 차징 중이다
      (switch Utilities|FlowControl|Switch|SwitchonE_Weapons (Variables|WeaponType|GetWeaponType)
        (:NewEnumerator0
          ;;[1 1 1] 오브젝트 스폰
          (bind _returnvalue (Game|SpawnActorfromClass "/Game/BowAndMusket/Weapons/Blueprints/NotGuns/BP_SeungjarGun_Pole.BP_SeungjarGun_Pole_C" (Math|Transform|MakeTransform (.location (Transformation|GetSocketTransform (Variables|Default|GetFrame) "FirePos" "RTS_World")) "0, 0, 0" "1,1,1") "Undefined" 0 0))
          (Utilities|IsValid _returnvalue
            (:Is%20Valid
              (bind _output_get (Variables|Default|SetPoleObject _returnvalue))
              (Transformation|AttachComponentToComponent _output_get (Variables|Default|GetFrame) "FirePos" "KeepWorld" "SnapToTarget" "KeepWorld" true)
              (bind _movement (Timeline|Pole_Movement Play)
                (:Update
                  (Utilities|IsValid (Variables|Default|GetPoleObject)
                    (:Is%20Valid
                      (Transformation|SetActorRelativeLocation (Variables|Default|GetPoleObject) (Math|Vector|Lerp(Vector) (Variables|Default|GetPole_BeginPos) (Variables|Default|GetPole_EndPos) _movement))
                      ;;[1 1 1] 차징 타임 1초마다  증가시킨다
                      (Utilities|FlowControl|Delay 1.0)
                      (Math|Float|IncrementFloat _chargingtimes
                        (:%20%20
                          (if (== _chargingtimes (Variables|Default|GetMaxChargingTimes))
                            ;;[1 1 1] 차징 바가 다 찼을 시
                            (Actor|DestroyActor (Variables|Default|GetPoleObject))
                            (Math|Integer|IncrementInt (Variables|GunChargingOrderFlags|GetChargingNumberCount)
                              (:%20%20
                                (Variables|GunChargingOrderFlags|SetIsCharging false) ; 차징 끝났다
                                (Variables|Default|SetAllowPoleMovement false) ; 차징 허용 안됨
                                ;;[1 0 0.03529] 차징 상태 업데이트(총기에 따라 다른 장전 메커니즘을 가집니다
                                (CallFunction|UpdateChargingSequence)))))))))))))
        (:NewEnumerator2
          (bind _returnvalue_2 (Game|SpawnActorfromClass "/Game/BowAndMusket/Weapons/Blueprints/NotGuns/BP_Pole.BP_Pole_C" (Math|Transform|MakeTransform (.location (Transformation|GetSocketTransform (Variables|Default|GetFrame) "FirePos" "RTS_World")) "0, 0, 0" "1,1,1") "Undefined" 0 0))
          (Utilities|IsValid _returnvalue_2
            (:Is%20Valid
              (bind _output_get_2 (Variables|Default|SetPoleObject _returnvalue_2))
              (Transformation|AttachComponentToComponent _output_get_2 (Variables|Default|GetFrame) "FirePos" "KeepWorld" "SnapToTarget" "SnapToTarget" true)
              (Timeline|Pole_Movement Play))))
        (:NewEnumerator3
          (bind _returnvalue_3 (Game|SpawnActorfromClass "/Game/BowAndMusket/Weapons/Blueprints/NotGuns/BP_CannonBall_Pole.BP_CannonBall_Pole_C" (Math|Transform|MakeTransform (.location (Transformation|GetSocketTransform (Variables|Default|GetFrame) "FirePos" "RTS_World")) "0, 0, 0" "1,1,1") "Undefined" 0 0))
          (Utilities|IsValid _returnvalue_3
            (:Is%20Valid
              (bind _output_get_3 (Variables|Default|SetPoleObject _returnvalue_3))
              (Transformation|AttachComponentToComponent _output_get_3 (Variables|Default|GetFrame) "FirePos" "KeepWorld" "SnapToTarget" "SnapToTarget" true)
              (Timeline|Pole_Movement Play))))))))

(event Custom|ReleaseTrigger
  ;[1 0.2849 0.5455] 코어 - 오브젝트 컨트롤
  ;;[1 1 1] 기타 이벤트 / 차일드에서 구현
  ;;;[1 1 1] Musket 사용 이벤트
)

(event EventBeginPlay
  (bind _chargingbarwidget (Variables|Default|GetChargingBarWidget))
  ;[1 1 1] BeginPlay
  (Variables|Default|SetFrameOffset (Variables|/Script/Engine.SceneComponent|GetRelativeRotation (Variables|Default|GetFrame)))
  (Variables|Default|SetInitialThrustStrength (Variables|/Script/Engine.PhysicsThrusterComponent|GetThrustStrength (Variables|Default|GetPhysicsThruster)))
  (bind _aswb_charging_bar (Utilities|Casting|CastToWB_ChargingBar (UserInterface|GetUserWidgetObject _chargingbarwidget)))
  (Variables|/Game/BowAndMusket/UMG/WB_ChargingBar.WB_ChargingBar_C|SetParentGunActor _aswb_charging_bar self)
  (Rendering|SetVisibility _chargingbarwidget false false)
  ;;[1 1 1] UI 엑터 가져오기
  (bind _outactors (Actor|GetAllActorsOfClass "/Game/BowAndMusket/Blueprints/BP_UMG_ExperenceMap.BP_UMG_ExperenceMap_C"))
  (Variables|Default|SetUIActors _outactors))

(event EventTick
  (params (DeltaSeconds :type Float%20%28single-precision%29))
  ;[1 1 1] 위치 프레임에 따라 재설정
  (Transformation|SetWorldLocation (Variables|Default|GetTriggerBoxParent) (Transformation|GetSocketLocation (Variables|Default|GetFrame) "Root") false false))

(fn ConstructionScript
  (bind _frame (Variables|Default|GetFrame))
  (bind _physicsthruster (Variables|Default|GetPhysicsThruster))
  (bind _frame_2 (Variables|Default|GetFrame))
  (bind _returnvalue (Transformation|GetSocketTransform _frame_2 "FirePos" "RTS_World"))
  (bind _returnvalue_2 (Transformation|GetSocketTransform _frame "Root" "RTS_World"))
  (bind (_location _rotation) (Math|Transform|BreakTransform _returnvalue))
  (Transformation|SetWorldLocationAndRotation (Variables|Default|GetTriggerBoxParent) (.location _returnvalue_2) (.rotation _returnvalue_2) false false)
  (Utilities|FlowControl|Sequence
    (:then_0
      (for _array_element (Utilities|Array|MakeArray (Variables|Default|GetChargingTrigger) (Variables|Default|Get2ndGrab) (Variables|Default|Get1ndGrab) (Variables|Default|GetFireTrigger) (Variables|Default|GetPowderTrigger) 0)
        (Utilities|IsValid _array_element
          (:Is%20Valid
            (Transformation|AttachComponentToComponent _array_element (Variables|Default|GetTriggerBoxParent) "None" "KeepRelative" "KeepRelative" "KeepRelative" true)
            (Transformation|AttachComponentToComponent (Variables|Default|GetGrabPosition) (Variables|Default|GetTriggerBoxParent) "None" "KeepRelative" "KeepRelative" "KeepRelative" true)))))
    (:then_1
      ;[1 1 1] 2Handed 그립 트리거 필요없으면 삭제
      (if (not (Variables|TriggerFlag|GetAllows2HandedGrip))
        (Components|DestroyComponent (Variables|Default|Get2ndGrab))))
    (:then_2
      ;[1 1 1] 화승 트리거 총기에 따라 필요없으면 삭제
      (if (not (Variables|TriggerFlag|GetAllowsFireTrigger))
        (Components|DestroyComponent (Variables|Default|GetFireTrigger))))
    (:then_3
      ;[1 1 1] 화약접시 트리거 총기에 따라 필요없으면 삭제
      (if (not (Variables|TriggerFlag|GetAllowsPowderTrigger))
        (Components|DestroyComponent (Variables|Default|GetPowderTrigger))))
    (:then_4
      ;[1 1 1] Recoil
      (Transformation|SetWorldLocationAndRotation _physicsthruster _location (Math|Rotator|CombineRotators "-45.000000, 0, 0" _rotation) false false)
      (Transformation|AttachComponentToComponent _physicsthruster (Variables|Default|GetFrame) "FirePos" "SnapToTarget" "KeepWorld" "SnapToTarget" true))))

(fn ActivateSpawnedBullet
  (params (SpawnedProjectile :type BP%20Projectile%20Base%20Object%20Reference))
  (Physics|SetSimulatePhysics (Variables|/Game/BowAndMusket/Weapons/Blueprints/NotGuns/Projectiles/BP_ProjectileBase.BP_ProjectileBase_C|GetBullet SpawnedProjectile) true)
  (Collision|IgnoreActorwhenMoving (Variables|/Game/BowAndMusket/Weapons/Blueprints/NotGuns/Projectiles/BP_ProjectileBase.BP_ProjectileBase_C|GetSphere SpawnedProjectile) self true)
  (Default|BulletOnly SpawnedProjectile) ; 총알 발사
  (Components|Activation|Activate (Variables|/Game/BowAndMusket/Weapons/Blueprints/NotGuns/Projectiles/BP_ProjectileBase.BP_ProjectileBase_C|GetProjectileMovement SpawnedProjectile) false))

(fn BulletSpawn
  (bind _weaponfireposition (Variables|Default|GetWeaponFirePosition))
  (bind _weaponfireposition_2 (Variables|Default|GetWeaponFirePosition))
  (bind _weaponfireposition_3 (Variables|Default|GetWeaponFirePosition))
  (bind _spawned_projectile (Variables|Default|GetSpawned%20Projectile))
  (bind (_location _rotation) (Math|Transform|BreakTransform _weaponfireposition_2))
  (bind (_location_2 _rotation_2) (Math|Transform|BreakTransform _weaponfireposition))
  (bind (_location_3 _rotation_3) (Math|Transform|BreakTransform _weaponfireposition_3))
  (Utilities|IsValid _spawned_projectile
    (:Is%20Valid
      ;[1 1 1] 비격진천뢰의 경우 - 프로젝타일이 무기에 붙어있음, 없애고 사격을 위해 재스폰한다
      (Actor|DestroyActor _spawned_projectile))
    (:Is%20Not%20Valid
      _))
  (switch Utilities|FlowControl|Switch|SwitchonE_Weapons (Variables|WeaponType|GetWeaponType)
    (:NewEnumerator0
      (bind _returnvalue (Game|SpawnActorfromClass "/Game/BowAndMusket/Weapons/Blueprints/NotGuns/Projectiles/BP_SeungjergunProjectile.BP_SeungjergunProjectile_C" (Math|Transform|MakeTransform _location _rotation "1,1,1") "Undefined" 0 0)) ; 총알 스폰
      (return _returnvalue))
    (:NewEnumerator2
      (bind _returnvalue_2 (Game|SpawnActorfromClass "/Game/BowAndMusket/Weapons/Blueprints/NotGuns/Projectiles/BP_ProjectileBase.BP_ProjectileBase_C" (Math|Transform|MakeTransform _location_3 _rotation_3 "1,1,1") "Undefined" 0 0)) ; 총알 스폰
      (return _returnvalue_2))
    (:NewEnumerator3
      (bind _returnvalue_3 (Game|SpawnActorfromClass "/Game/BowAndMusket/Weapons/Blueprints/NotGuns/Projectiles/BP_CannonBallProjectile.BP_CannonBallProjectile_C" (Math|Transform|MakeTransform _location_2 _rotation_2 "1,1,1") "Undefined" 0 0)) ; 총알 스폰
      (Collision|SetCollisionEnabled (Variables|/Game/BowAndMusket/Weapons/Blueprints/NotGuns/Projectiles/BP_ProjectileBase.BP_ProjectileBase_C|GetBullet _returnvalue_3) "NoCollision")
      (return _returnvalue_3))))