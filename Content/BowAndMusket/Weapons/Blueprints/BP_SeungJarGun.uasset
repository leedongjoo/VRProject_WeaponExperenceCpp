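; Seungja-chongtong hand cannon, a two-grip child weapon with a staged muzzle-loading and fuse-firing procedure.
; GunChargingSequence tracks powder, mud wad, bullet and mud seal, with ChargingNumberCount marking each completed ramming stage.
; The final stage enables the fire trigger; GetFire attaches BP_Fire to the rope socket, then after a delay removes it and fires with recoil.
; The construction script snaps grips, triggers, rope and charging-bar widget to Frame sockets.
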(event EventGetFire
  (bind _frame (Variables|Default|GetFrame))
  (bind _returnvalue (Transformation|GetSocketTransform _frame "FireRopePos" "RTS_World"))
  ;[1 1 1] 불 스폰 후 어태치
  (if (Variables|Default|GetFireAttachable)
    (bind _returnvalue_2 (Game|SpawnActorfromClass "/Game/BowAndMusket/Weapons/Blueprints/NotGuns/BP_Fire.BP_Fire_C" (Math|Transform|MakeTransform (.location _returnvalue) (.rotation _returnvalue) "0.500000,0.500000,0.500000") "Undefined" 0 0))
    (bind _output_get (Variables|Default|SetAttachedFire _returnvalue_2))
    (Transformation|AttachComponentToComponent _output_get (Variables|Default|GetFrame) "FireRopePos" "SnapToTarget" "SnapToTarget" "KeepWorld" true)
    (Variables|Default|SetFireAttachable false) ; 이제 불 부착 불가능
    (Utilities|IsValid (Variables|Default|GetAttachedFire) ; 불이 부착 시
      (:Is%20Valid
        (bind _structout (Utilities|Struct|SetmembersinS_GunChargingSequence (Variables|Default|GetGunChargingSequence) true)) ; 최종 장전 완료
        (CallFunction|SendSequence _structout)
        ;[1 0.315 0.7774] 격발 메커니즘 - 불을 붙이면 3초 뒤 격발이 시작된다
        (Utilities|FlowControl|Delay 3.0)
        (CallFunction|DeleteFire) ; 불 소멸
        (CallFunction|SpawnEmitterandRecoil) ; 총알 발사
      ))))

(event EventDeleteFire
  (bind _attachedfire (Variables|Default|GetAttachedFire))
  ;[1 1 1] 불 소멸
  (|CallParentFunction)
  (Utilities|IsValid _attachedfire
    (:Is%20Valid
      (Actor|DestroyActor _attachedfire)
      (Variables|Default|SetFireAttachable true))))

(event EventSpawnGrabPositionObjects
  ;[1 1 1] 스폰된 그랩 포지션 오브젝트 무기에 맞게 크기 변경
)

(event EventGetGunPowder
  ;[1 1 1] 승자총통의 장전 절차
  ;;[1 0 0.03529] 첫 번째(공통) - 총구를 세척하고 총구에 화약과 토격을 삽입한다
  (|CallParentFunction))

(event EventGetBullet
  (bind _gunchargingsequence (Variables|Default|GetGunChargingSequence))
  ;[1 1 1] 승자총통의 장전 절차
  ;;[1 0 0.03529] 두 번째 - 총알을 삽입하고 토격으로 총알을 밀봉한다 - 총구 장전 완료
  (|CallParentFunction)
  (if (.2ndFPowderChargingComplete (Utilities|Struct|BreakS_GunChargingSequence _gunchargingsequence)) ; 2번째 차징 완료시 (순서에 따라)
    ;;;[1 1 1] 총알 존재X, 3번째 차징 완료되지 않았을 때
    (if (not (and (.HasBullet (Utilities|Struct|BreakS_GunChargingSequence _gunchargingsequence)) (.3ndBulletChargingComplete (Utilities|Struct|BreakS_GunChargingSequence _gunchargingsequence))))
      (bind _structout (Utilities|Struct|SetmembersinS_GunChargingSequence _gunchargingsequence true)) ; 총알을 획득합니다
      (CallFunction|SendSequence _structout))))

(event EventBeginPlay
  ;[1 1 1] BeginPlay
  (|CallParentFunction)
  (CallFunction|SpawnGrabPositionObjects))

(event EventUpdateChargingSequence
  (bind _gunchargingsequence (Variables|Default|GetGunChargingSequence))
  ;[1 1 1] 승자총통의 장전 절차
  (Utilities|FlowControl|Sequence
    (:then_0
      (switch int (Variables|Default|GetChargingNumberCount) ; 차징 횟수에 따라 순서 구별
        (:1
          ;;[1 0 0.03529] 첫 번째(공통) - 총구를 세척하고 총구에 화약과 토격을 삽입한다
          (bind _structout (Utilities|Struct|SetmembersinS_GunChargingSequence _gunchargingsequence true))
          (CallFunction|SendSequence _structout))
        (:2
          ;;[1 0 0.03529] 두 번째 - 총알을 삽입하고 토격으로 총알을 밀봉한다 - 총구 장전 완료
          (bind _structout_2 (Utilities|Struct|SetmembersinS_GunChargingSequence _gunchargingsequence true)) ; 화약 다지기 완료
          (CallFunction|SendSequence _structout_2))
        (:3
          ;;[1 0 0.03529] 세 번째 - 불을 붙인 후 격발한다
          (bind _structout_3 (Utilities|Struct|SetmembersinS_GunChargingSequence _gunchargingsequence true)) ; 최종 장전 완료
          (CallFunction|SendSequence _structout_3)
          (CallFunction|FireTriggerCollisionToggle "QueryOnly") ; 파이어 트리거 콜리전 활성화
        )))))

(event EventGetMud
  (bind _gunchargingsequence (Variables|Default|GetGunChargingSequence))
  ;[1 1 1] 승자총통의 장전 절차
  ;;[1 0 0.03529] 첫 번째(공통) - 총구를 세척하고 총구에 화약과 토격을 삽입한다
  ;;;[1 1 1] 첫 번째 순서에 따라
  (|CallParentFunction)
  (if (and (.InitialChargingComplete (Utilities|Struct|BreakS_GunChargingSequence (Variables|Default|GetGunChargingSequence))) (not (.2ndFPowderChargingComplete (Utilities|Struct|BreakS_GunChargingSequence (Variables|Default|GetGunChargingSequence)))))
    (if (.HasFiringPowder (Utilities|Struct|BreakS_GunChargingSequence (Variables|Default|GetGunChargingSequence))) ; 화약이 존재한다면
      (if (not (.HasFirstPowderMud (Utilities|Struct|BreakS_GunChargingSequence (Variables|Default|GetGunChargingSequence)))) ; 토격이 존재하지 않는다면
        (bind _structout (Utilities|Struct|SetmembersinS_GunChargingSequence (Variables|Default|GetGunChargingSequence) true)) ; 토격 삽입
        (CallFunction|SendSequence _structout)
        (Variables|Default|SetFirstMudObjectDestroy true) ; 삽입 성공시 삭제 가능
        (CallFunction|RechargebyChargingSequence) ; 장전 상태 초기화
      ))
    (else
      ;;[1 0 0.03529] 두 번째 - 총알을 삽입하고 토격으로 총알을 밀봉한다 - 총구 장전 완료
      ;;;[1 1 1] 토격으로 총알을 밀봉한다
      (if (.HasBullet (Utilities|Struct|BreakS_GunChargingSequence (Variables|Default|GetGunChargingSequence))) ; 총알이 존재한다면
        (if (not (.HasSecondPowderMud (Utilities|Struct|BreakS_GunChargingSequence _gunchargingsequence))) ; 토격이 존재하지 않는다면
          (bind _structout_2 (Utilities|Struct|SetmembersinS_GunChargingSequence _gunchargingsequence true)) ; 토격 삽입
          (CallFunction|SendSequence _structout_2)
          (Variables|Default|SetFirstMudObjectDestroy true) ; 삽입 성공시 삭제 가능
          (CallFunction|RechargebyChargingSequence) ; 다시 차징 허용(화약 다지기)
        )))))

(fn ConstructionScript
  (bind _frame (Variables|Default|GetFrame))
  (bind _frame_2 (Variables|Default|GetFrame))
  (bind _frame_3 (Variables|Default|GetFrame))
  (bind _frame_4 (Variables|Default|GetFrame))
  (bind _rope (Variables|Default|GetRope))
  (bind _frame_5 (Variables|Default|GetFrame))
  (bind _returnvalue (Transformation|GetSocketTransform _frame_5 "OneHandGrip" "RTS_World"))
  (bind _returnvalue_2 (Transformation|GetSocketTransform _frame_2 "FireTrigger" "RTS_World"))
  (bind _returnvalue_3 (Transformation|GetSocketTransform _frame_3 "FireTrigger" "RTS_World"))
  (bind _returnvalue_4 (Transformation|GetSocketTransform _frame "TwoHandGrip" "RTS_World"))
  (bind _returnvalue_5 (Transformation|GetSocketTransform _frame_4 "FirePos" "RTS_World"))
  (bind (_location _rotation) (Math|Transform|BreakTransform _returnvalue))
  (bind (_location_2 _rotation_2) (Math|Transform|BreakTransform _returnvalue_2))
  (bind (_location_3 _rotation_3) (Math|Transform|BreakTransform _returnvalue_3))
  (bind (_location_4 _rotation_4) (Math|Transform|BreakTransform _returnvalue_4))
  (bind (_location_5 _rotation_5) (Math|Transform|BreakTransform _returnvalue_5))
  (|CallParentFunction)
  (Transformation|SetWorldLocationAndRotation (Variables|Default|Get2ndGrab) _location_4 _rotation_4 false false)
  (Transformation|SetWorldLocationAndRotation (Variables|Default|Get1ndGrab) _location _rotation false false)
  (Transformation|SetWorldLocationAndRotation (Variables|Default|GetFireTrigger) _location_2 _rotation_2 false false)
  (Transformation|SetWorldLocationAndRotation (Variables|Default|GetChargingTrigger) _location_5 _rotation_5 false false)
  (Transformation|SetWorldLocationAndRotation _rope _location_3 _rotation_3 false false)
  (Transformation|AttachComponentToComponent _rope (Variables|Default|GetFrame) "FireTrigger" "SnapToTarget" "SnapToTarget" "KeepWorld" true)
  (Transformation|SetWorldLocationAndRotation (Variables|Default|GetChargingBarWidget) (.Location (Math|Transform|BreakTransform (Transformation|GetSocketTransform (Variables|Default|GetFrame) "FirePos" "RTS_World"))) "90.000000, 0, 0" false false))